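; Vertical bumper that launches the player along the Z axis on contact.
; A timeline restarts itself on finish from BeginPlay onward, continuously animating the relative Z location of Sphere1.
; When BP_Player overlaps the Collider, it calls the player's BumpPlayer with a Z-only launch velocity set by a variable and plays a 2D sound.
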(event OnComponentBeginOverlap(Collider)
  (params (OverlappedComponent :type Primitive%20Component%20Object%20Reference) (OtherActor :type Actor%20Object%20Reference) (OtherComp :type Primitive%20Component%20Object%20Reference) (OtherBodyIndex :type Integer) (bFromSweep :type Boolean) (SweepResult :type Hit%20Result%20Structure%20%28by%20ref%29))
  (bind _asbp_player (Utilities|Casting|CastToBP_Player OtherActor))
  (Default|BumpPlayer _asbp_player (Math|Vector|MakeVector 0.0 0.0 (Variables|ImpulseForce|GetLaunchVelocityZ)))
  (Audio|PlaySound2D "/Engine/VREditor/Sounds/UI/Object_PickUp.Object_PickUp" 1.0 1.0 0.0 0 0))

(event Custom|PlayAnimStart
  (bind _zaxis (Timeline|Timeline PlayFromStart)
    (:Update
      (Transformation|SetRelativeLocation (Variables|Default|GetSphere1) (Math|Vector|MakeVector 0.0 0.0 _zaxis) false false))
    (:Finished
      (CallFunction|PlayAnimStart))))

(event EventBeginPlay
  (CallFunction|PlayAnimStart))

(fn ConstructionScript)