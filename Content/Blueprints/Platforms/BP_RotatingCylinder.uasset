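; BP_RotatingCylinder is a spinning platform obstacle that bumps the player on contact.
; At BeginPlay it randomly picks a yaw direction and speed for its RotatingMovement component.
; When BP_Player begins overlapping the Capsule, it calls BumpPlayer with a vector built from that rotation rate and the ForceX and ForceY values.
; The vertical component gets a fixed offset scaled by ForceZ, adding lift to the bump.
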(event OnComponentBeginOverlap(Capsule)
  (params (OverlappedComponent :type Primitive%20Component%20Object%20Reference) (OtherActor :type Actor%20Object%20Reference) (OtherComp :type Primitive%20Component%20Object%20Reference) (OtherBodyIndex :type Integer) (bFromSweep :type Boolean) (SweepResult :type Hit%20Result%20Structure%20%28by%20ref%29))
  (bind _rotatingmovement (Variables|Default|GetRotatingMovement))
  (bind _forcex (Variables|ForceImpulse|GetForceX))
  (bind _forcey (Variables|ForceImpulse|GetForceY))
  (bind _returnvalue (Math|Vector|MakeVector _forcex _forcey 0.0))
  (bind _rotationrate (Variables|/Script/Engine.RotatingMovementComponent|GetRotationRate _rotatingmovement))
  (bind _returnvalue_2 (* _rotationrate _returnvalue))
  (bind (_x _y _z) (Math|Vector|BreakVector _returnvalue_2))
  (bind _asbp_player (Utilities|Casting|CastToBP_Player OtherActor))
  (Default|BumpPlayer _asbp_player (Math|Vector|MakeVector _x _y (* (+ _z 5e+01) (Variables|ForceImpulse|GetForceZ)))))

(event EventBeginPlay
  ;[1 1 1] Set random speed rotation rate
  (if (== (Math|Random|RandomIntegerinRange 0 1) 0)
    (Variables|/Script/Engine.RotatingMovementComponent|SetRotationRate (Variables|Default|GetRotatingMovement) (Math|Rotator|MakeRotator 0.0 0.0 (Math|Random|RandomFloatinRange 5e+01 1.5e+02)))
    (else
      (Variables|/Script/Engine.RotatingMovementComponent|SetRotationRate (Variables|Default|GetRotatingMovement) (Math|Rotator|MakeRotator 0.0 0.0 (Math|Random|RandomFloatinRange -5e+01 -1.5e+02))))))

(fn ConstructionScript)