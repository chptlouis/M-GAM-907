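; Interactable actor that toggles a cube between solid and hidden, acting like a simple openable door or barrier.
; A sphere trigger shows a widget while something overlaps it and hides it on exit.
; The Interact event flips IsOpen, plays a click sound, and switches the cube's visibility and collision to match.
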(event OnComponentBeginOverlap(Sphere)
  (params (OverlappedComponent :type Primitive%20Component%20Object%20Reference) (OtherActor :type Actor%20Object%20Reference) (OtherComp :type Primitive%20Component%20Object%20Reference) (OtherBodyIndex :type Integer) (bFromSweep :type Boolean) (SweepResult :type Hit%20Result%20Structure%20%28by%20ref%29))
  (Rendering|SetVisibility (Variables|Default|GetWidget) true false))

(event OnComponentEndOverlap(Sphere)
  (params (OverlappedComponent :type Primitive%20Component%20Object%20Reference) (OtherActor :type Actor%20Object%20Reference) (OtherComp :type Primitive%20Component%20Object%20Reference) (OtherBodyIndex :type Integer))
  (Rendering|SetVisibility (Variables|Default|GetWidget) false false))

(event EventInteract
  (if (not (Variables|Default|GetisOpen))
    (Variables|Default|SetisOpen true)
    (Audio|PlaySound2D "/Engine/VREditor/Sounds/UI/Click_on_Button.Click_on_Button" 1.0 1.0 0.0 0 0)
    (Rendering|SetVisibility (Variables|Default|GetCube1) false false)
    (Collision|SetCollisionEnabled (Variables|Default|GetCube1) "NoCollision")
    (else
      (Variables|Default|SetisOpen false)
      (Audio|PlaySound2D "/Engine/VREditor/Sounds/UI/Click_on_Button.Click_on_Button" 1.0 1.0 0.0 0 0)
      (Rendering|SetVisibility (Variables|Default|GetCube1) true false)
      (Collision|SetCollisionEnabled (Variables|Default|GetCube1) "QueryAndPhysics"))))

(fn ConstructionScript)