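; BP_BoxCrash is a configurable level prop whose mesh slides to an end position while a Character stands in its Box trigger.
; Entering plays a sound and runs the MoveBox timeline, lerping from the starting relative location to EndLocation, paced by DurationSeconds; leaving reverses it.
; The construction script applies the chosen mesh, scale and rotation to both the moving mesh and a reference mesh placed at EndLocation.
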(event OnComponentBeginOverlap(Box)
  (params (OverlappedComponent :type Primitive%20Component%20Object%20Reference) (OtherActor :type Actor%20Object%20Reference) (OtherComp :type Primitive%20Component%20Object%20Reference) (OtherBodyIndex :type Integer) (bFromSweep :type Boolean) (SweepResult :type Hit%20Result%20Structure%20%28by%20ref%29))
  (Utilities|Casting|CastToCharacter OtherActor)
  (Audio|PlaySound2D "/Engine/VREditor/Sounds/UI/Dockable_Window_Close.Dockable_Window_Close" 1.0 1.0 0.0 0 0)
  (Components|Timeline|SetPlayRate (Variables|Default|GetMove%20Box) (/ 1.0 (Variables|Default|GetDuration%20%28seconds%29)))
  (bind _move_track (Timeline|Move%20Box Play)
    (:Update
      (Transformation|SetRelativeLocation (Variables|Default|GetBoxMeshInit) (Math|Vector|Lerp(Vector) (Variables|Default|GetStart%20Location) (Variables|Default|GetEnd%20Location) _move_track) false false))))

(event OnComponentEndOverlap(Box)
  (params (OverlappedComponent :type Primitive%20Component%20Object%20Reference) (OtherActor :type Actor%20Object%20Reference) (OtherComp :type Primitive%20Component%20Object%20Reference) (OtherBodyIndex :type Integer))
  (Utilities|Casting|CastToCharacter OtherActor)
  (Components|Timeline|SetPlayRate (Variables|Default|GetMove%20Box) (/ 1.0 (Variables|Default|GetDuration%20%28seconds%29)))
  (bind _move_track (Timeline|Move%20Box Reverse)
    (:Update
      (Transformation|SetRelativeLocation (Variables|Default|GetBoxMeshInit) (Math|Vector|Lerp(Vector) (Variables|Default|GetStart%20Location) (Variables|Default|GetEnd%20Location) _move_track) false false))))

(event EventBeginPlay
  (Variables|Default|SetStart%20Location (Variables|/Script/Engine.SceneComponent|GetRelativeLocation (Variables|Default|GetBoxMeshInit))))

(fn ConstructionScript
  (bind _boxmeshinit (Variables|Default|GetBoxMeshInit))
  (bind _boxmeshendreference (Variables|Default|GetBoxMeshEndReference))
  (bind _boxmesh (Variables|Default|GetBoxMesh))
  (Components|StaticMesh|SetStaticMesh _boxmeshinit _boxmesh)
  (Components|StaticMesh|SetStaticMesh _boxmeshendreference _boxmesh)
  (Transformation|SetRelativeScale3D _boxmeshinit (Variables|Default|GetScale))
  (Transformation|SetRelativeRotation _boxmeshinit (Variables|Default|GetRotation) false false)
  (Transformation|SetRelativeLocation _boxmeshendreference (Variables|Default|GetEnd%20Location) false false))